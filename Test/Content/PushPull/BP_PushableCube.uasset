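; BP_PushableCube is a cube that the third-person character can push and pull along its horizontal axes.
; Box overlap registers the cube on the character and enables interaction; ending overlap only prints, clearing nothing.
; While the character interacts, Tick converts MoveY and MoveX signs into fixed-speed SpeedDirection calls.
; SpeedDirection eases the Cube component along its right (forward/back input) or forward (left/right) vector using VInterpTo, without sweeping.
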(event `self.ReceiveTick`
  (params (DeltaSeconds :type "Float (single-precision)"))
  (bind _as_bp_third_person_character (`self.As BP Third Person Character`))
  (bind _movey (`/Game/ThirdPerson/Blueprints/BP_ThirdPersonCharacter.MoveY` _as_bp_third_person_character))
  (bind _movex (`/Game/ThirdPerson/Blueprints/BP_ThirdPersonCharacter.MoveX` _as_bp_third_person_character))
  (bind _as_bp_third_person_character_2 (`self.As BP Third Person Character`)
    (:`then`
      (if (and (`/Game/ThirdPerson/Blueprints/BP_ThirdPersonCharacter.IsInteracting` _as_bp_third_person_character_2) (`/Game/ThirdPerson/Blueprints/BP_ThirdPersonCharacter.CanInteractBox` _as_bp_third_person_character_2))
        (`|ExecutionSequence`
          (:`then_0`
            (if (== _movey 0.0)
              (`KismetSystemLibrary.PrintString` "Is not moving FB" true true (struct :`G` 1.0 :`B` 0.296857 :`A` 1.0))
              (`self.SpeedDirection` false)
              (elif (>= _movey 0.1)
                (`KismetSystemLibrary.PrintString` "MOVING UP" true true (struct :`G` 1.0 :`B` 0.296857 :`A` 1.0))
                (`self.SpeedDirection` true 15.0)
                (else
                  (`KismetSystemLibrary.PrintString` "MOVING DOWN" true true (struct :`G` 1.0 :`B` 0.296857 :`A` 1.0))
                  (`self.SpeedDirection` true -15.0)))))
          (:`then_1`
            (if (== _movex 0.0)
              (`KismetSystemLibrary.PrintString` "Is not movingRL" true true (struct :`G` 1.0 :`B` 0.296857 :`A` 1.0))
              (`self.SpeedDirection` false)
              (elif (>= _movex 0.1)
                (`KismetSystemLibrary.PrintString` "MOVING RIGHT" true true (struct :`G` 1.0 :`B` 0.296857 :`A` 1.0))
                (`self.SpeedDirection` false -15.0)
                (else
                  (`KismetSystemLibrary.PrintString` "MOVING LEFT" true true (struct :`G` 1.0 :`B` 0.296857 :`A` 1.0))
                  (`self.SpeedDirection` false 15.0))))))))
    (:`else`)))

(event `self.Box.OnComponentBeginOverlap`
  (params (OverlappedComponent :type "PrimitiveComponent Object Reference") (OtherActor :type "Actor Object Reference") (OtherComp :type "PrimitiveComponent Object Reference") (OtherBodyIndex :type Integer) (bFromSweep :type Boolean) (SweepResult :type "HitResult Structure (by ref)"))
  (bind _output_get (set `self.As BP Third Person Character` (cast `/Game/ThirdPerson/Blueprints/BP_ThirdPersonCharacter` OtherActor :!pure true)))
  (set `/Game/ThirdPerson/Blueprints/BP_ThirdPersonCharacter.BP_PushableCube` self _output_get)
  (set `/Game/ThirdPerson/Blueprints/BP_ThirdPersonCharacter.CanInteractBox` true _output_get)
  (`KismetSystemLibrary.PrintString` "IS OVERLAPING" true true (struct :`R` 0.966025 :`G` 0.044729 :`B` 1.0 :`A` 1.0)))

(event `self.Box.OnComponentEndOverlap`
  (params (OverlappedComponent :type "PrimitiveComponent Object Reference") (OtherActor :type "Actor Object Reference") (OtherComp :type "PrimitiveComponent Object Reference") (OtherBodyIndex :type Integer))
  (`KismetSystemLibrary.PrintString` "NOT OVERLAPING" true true (struct :`R` 1.0 :`G` 0.31786 :`A` 1.0)))

(fn `UserConstructionScript`)