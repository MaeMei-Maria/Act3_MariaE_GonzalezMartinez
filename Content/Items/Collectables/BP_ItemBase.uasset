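; BP_ItemBase is the base actor for collectable items in the world, spinning steadily each tick.
; Its box overlap sets an Object reference on BP_Character when the character enters and clears it on exit.
; It holds item data assignable through SetItemData, packages it with a quantity via MakeItemForInventory for the inventory, and exposes a DestroyActor event to remove itself.
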(event `self.Box.OnComponentBeginOverlap`
  (params (OverlappedComponent :type "PrimitiveComponent Object Reference") (OtherActor :type "Actor Object Reference") (OtherComp :type "PrimitiveComponent Object Reference") (OtherBodyIndex :type Integer) (bFromSweep :type Boolean) (SweepResult :type "HitResult Structure (by ref)"))
  (bind _asbp_character (cast `/Game/ThirdPerson/Blueprints/BP_Character` OtherActor :!pure true))
  (`/Engine/EditorBlueprintResources/StandardMacros.IsValid` _asbp_character
    (:`Is Valid`
      (set `/Game/ThirdPerson/Blueprints/BP_Character.Object` (`self.Object`) _asbp_character))))

(event `self.Box.OnComponentEndOverlap`
  (params (OverlappedComponent :type "PrimitiveComponent Object Reference") (OtherActor :type "Actor Object Reference") (OtherComp :type "PrimitiveComponent Object Reference") (OtherBodyIndex :type Integer))
  (set `/Game/ThirdPerson/Blueprints/BP_Character.Object` null (cast `/Game/ThirdPerson/Blueprints/BP_Character` OtherActor :!pure true)))

(event `self.ReceiveTick`
  (params (DeltaSeconds :type "Float (single-precision)"))
  (`self.K2_AddActorLocalRotation` (struct :`Yaw` 5.0)))

(event `/Game/UI/Inventory/Components/Interfaces/I_Interactable.SetItemData`
  (params (ItemData :type "/Game/UI/Inventory/Components/Data/PDA_ItemData Object Reference"))
  (set `self.ItemData` ItemData))

(event `/Game/UI/Inventory/Components/Interfaces/I_Interactable.DestroyActor`
  (`self.K2_DestroyActor`))

(fn `MakeItemForInventory`
  (returns (ItemToAdd :type "/Game/UI/Inventory/Components/Structures/S_InventorySlot Structure"))
  (return (`/Game/UI/Inventory/Components/Library/BFL_Inventory.MakeItemToAdd` (`|ConvertAsset` (`self.ItemData`)) (`self.Quantity`))))

(fn `UserConstructionScript`)