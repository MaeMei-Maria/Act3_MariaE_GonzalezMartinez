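; BP_WeaponBase is a base weapon item that deals melee-style damage to characters and destroys itself on unequip.
; Attack runs only with authority, doing a single sphere trace for pawns at a weapon mesh socket, with identical start and end points.
; The hit actor, cast to BP_Character, receives the weapon's damage with the weapon as causer.
; The trace draws timed debug shapes.
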(fn `Attack`
  (bind _returnvalue (`SceneComponent.GetSocketLocation` (`self.WeaponMesh`) (`self.SocketName`)))
  (`/Engine/EditorBlueprintResources/ActorMacros.Switch Has Authority`
    (:`Authority`
      (bind _outhit (`KismetSystemLibrary.SphereTraceSingleForObjects` :`Start` _returnvalue :`End` _returnvalue :`Radius` (`self.RadiusOfDamage`) :`ObjectTypes` (`|MakeArray` "ObjectTypeQuery3" :!type "EObjectTypeQuery Enum") :`DrawDebugType` "ForDuration"))
      (`GameplayStatics.ApplyDamage` (cast `/Game/Character/Blueprints/BP_Character` (`.HitActor` (`GameplayStatics.BreakHitResult` _outhit)) :!pure true) (`self.Damage`) null self))))

(fn `OnUnequip`
  (`self.K2_DestroyActor`))

(fn `UserConstructionScript`)