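; BP_Hammer is a usable hammer item that deals damage to a character at its strike point.
; CE_UseHammer runs only on authority, performing a stationary sphere trace for Pawn objects at the Hammer's DamageSocket, sized by RadiusOfDamage.
; The single hit actor is cast to BP_Character and receives Damage through ApplyDamage, with the hammer as damage causer.
; Debug drawing of the trace is enabled.
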(event `self.ReceiveActorBeginOverlap`
  (params (OtherActor :type "Actor Object Reference")))

(event `CE_UseHammer`
  (bind _returnvalue (`SceneComponent.GetSocketLocation` (`self.Hammer`) "DamageSocket"))
  (`/Engine/EditorBlueprintResources/ActorMacros.Switch Has Authority`
    (:`Authority`
      (bind _outhit (`KismetSystemLibrary.SphereTraceSingleForObjects` :`Start` _returnvalue :`End` _returnvalue :`Radius` (`self.RadiusOfDamage`) :`ObjectTypes` (`|MakeArray` "ObjectTypeQuery3" :!type "EObjectTypeQuery Enum") :`DrawDebugType` "ForDuration"))
      (`GameplayStatics.ApplyDamage` (cast `/Game/ThirdPerson/Blueprints/BP_Character` (`.HitActor` (`GameplayStatics.BreakHitResult` _outhit)) :!pure true) (`self.Damage`) null self))))

(fn `UserConstructionScript`)