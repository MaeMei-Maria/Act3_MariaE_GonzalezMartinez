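; Game state that runs the pre-fight countdown and presents the fight start and the winner.
; On the authority, Tick decrements TotalGameCount by one per tick until it reaches zero, then sets FightPhase.
; FightPhase's RepNotify shows a "FIGHT!!" message through the first player controller's widget.
; WinnerPlayerState's RepNotify plays the winner montage, shows a final screen with the player's name and disables that character's movement.
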(event `self.ReceiveTick`
  (params (DeltaSeconds :type "Float (single-precision)"))
  (`/Engine/EditorBlueprintResources/ActorMacros.Switch Has Authority`
    (:`Authority`
      (if (!= (`self.TotalGameCount`) 0.0)
        (bind _result (`/Engine/EditorBlueprintResources/StandardMacros.DecrementFloat` (`self.TotalGameCount`))
          (:`  `
            (bind _output_get (set `self.TotalGameCount` _result))
            (if (<= _output_get 0.0)
              (set `self.FightPhase` true)
              (set `self.TotalGameCount` 0.0))))))))

(fn `OnRep_FightPhase`
  (`/Game/UI/WBP_PlayerHUD.ShowMessage` (`/Game/Character/Blueprints/BP_PlayerController.UserWidget` (cast `/Game/Character/Blueprints/BP_PlayerController` (`GameplayStatics.GetPlayerController` 0) :!pure true)) "FIGHT!!"))

(fn `OnRep_WinnerPlayerState`
  (bind _winnerplayerstate (`self.WinnerPlayerState`))
  (bind _asbp_character (cast `/Game/Character/Blueprints/BP_Character` (`PlayerState.GetPawn` _winnerplayerstate) :!pure true))
  (`Character.PlayAnimMontage` _asbp_character "/Game/Character/CharacterVisual/Anim/AM_Winner.AM_Winner" 1.0 "None")
  (bind _returnvalue (`|CreateWidget` "/Game/UI/WBP_FinalScreen.WBP_FinalScreen_C" null (`KismetTextLibrary.Conv_TextToString` (`/Game/Character/Blueprints/BP_PlayerState.PlayerName` _winnerplayerstate))))
  (`UserWidget.AddToViewport` _returnvalue 0)
  (`CharacterMovementComponent.DisableMovement` (`Character.CharacterMovement` _asbp_character)))

(fn `UserConstructionScript`)